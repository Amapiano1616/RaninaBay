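; Twinmotion volumetric cloud actor that drives a VolumetricCloud component, sky sphere visibility and the MPC_VolumetricClouds material parameters.
; RefreshSettings, run on construction and CloudsUpdateSettings, converts artist controls into layer geometry, shaping, dissipation, albedo, cirrus and seeded random offsets.
; Tick accumulates cloud position and time from wind parameters in EnvironmentMaterialParameters, halting while paused or path tracing and resetting at zero cloud speed.
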(event Custom|CloudsUpdateSettings
  (CallFunction|RefreshSettings))

(event EventBeginPlay)

(event Collision|EventActorBeginOverlap
  (params (OtherActor :type Actor%20Object%20Reference)))

(event EventTick
  (params (DeltaSeconds :type Float%20%28single-precision%29))
  (CallFunction|UpdateCloudsRuntimeOffset DeltaSeconds))

(fn ConstructionScript
  (CallFunction|RefreshSettings))

(fn UpdateCloudsRuntimeOffset
  (params (deltatime :type Float%20%28double-precision%29))
  (LocalVariables|SetL_DeltaTime deltatime)
  (Utilities|FlowControl|Sequence
    (:then_0
      ;[1 0.7376 0] Initialize Constants from Material Parameter Collections
      (Utilities|FlowControl|Sequence
        (:then_0
          (bind _returnvalue (Rendering|Material|GetScalarParameterValue "/Game/Twinmotion/Environment/EnvironmentMaterialParameters.EnvironmentMaterialParameters" "CPS_VCloudsWindSpeedAdjust" :!class /Script/Engine.KismetMaterialLibrary))
          (LocalVariables|SetL_CloudsSpeedAdjust _returnvalue))
        (:then_1
          (bind _returnvalue_2 (Rendering|Material|GetScalarParameterValue "/Game/Twinmotion/Environment/EnvironmentMaterialParameters.EnvironmentMaterialParameters" "CPS_PathTracerActive" :!class /Script/Engine.KismetMaterialLibrary))
          (LocalVariables|SetL_PathtracerOff (- 1.0 _returnvalue_2)))
        (:then_2
          (bind _returnvalue_3 (Rendering|Material|GetScalarParameterValue "/Game/Twinmotion/Environment/EnvironmentMaterialParameters.EnvironmentMaterialParameters" "CPS_VegetationWindSpeed" :!class /Script/Engine.KismetMaterialLibrary))
          (LocalVariables|SetL_GlobalWindSpeed _returnvalue_3))
        (:then_3
          (bind _returnvalue_4 (Rendering|Material|GetVectorParameterValue "/Game/Twinmotion/Environment/EnvironmentMaterialParameters.EnvironmentMaterialParameters" "CPV3_WindDirection" :!class /Script/Engine.KismetMaterialLibrary))
          (LocalVariables|SetL_WindDirection _returnvalue_4))
        (:then_4
          (bind _returnvalue_5 (Rendering|Material|GetScalarParameterValue "/Game/Twinmotion/Environment/EnvironmentMaterialParameters.EnvironmentMaterialParameters" "CPS_TwinmotionPaused" :!class /Script/Engine.KismetMaterialLibrary))
          (LocalVariables|SetL_TMActive (Math|Float|Clamp(Float) (- 1.0 _returnvalue_5))))))
    (:then_1
      ;[0 0.521 1] Increment Cloud Position & Time Values
      (Variables|Default|SetCloudsRuntimeOffset (Math|Vector|SelectVector (+ (* (LocalVariables|GetL_WindDirection) (* (LocalVariables|GetL_GlobalWindSpeed) (LocalVariables|GetL_DeltaTime) (LocalVariables|GetL_PathtracerOff) (LocalVariables|GetL_CloudsSpeedAdjust) (Math|Float|MakeLiteralFloat 1e+04) (LocalVariables|GetL_TMActive))) (Variables|Default|GetCloudsRuntimeOffset)) "0, 0, 0" (> (LocalVariables|GetL_CloudsSpeedAdjust) 0.0)))
      (Variables|Default|SetCloudsTime (Math|Float|SelectFloat (+ (* (LocalVariables|GetL_PathtracerOff) (LocalVariables|GetL_DeltaTime) (LocalVariables|GetL_CloudsSpeedAdjust) (LocalVariables|GetL_TMActive)) (Variables|Default|GetCloudsTime)) 0.0 (> (LocalVariables|GetL_CloudsSpeedAdjust) 0.0))))
    (:then_2
      ;[0 0.07825 1] Apply Cloud Position & Time Values
      (Rendering|Material|SetVectorParameterValue "/Game/Twinmotion/Environment/VolumetricClouds/Resources/Materials/MPC_VolumetricClouds.MPC_VolumetricClouds" "Position" (Math|Conversions|ToLinearColor(Vector) (+ (Variables|Default|GetCloudsRuntimeOffset) (Math|Conversions|ToVector(Vector2D) (Variables|Default|GetStaticOffset)))) :!class /Script/Engine.KismetMaterialLibrary)
      (Rendering|Material|SetScalarParameterValue "/Game/Twinmotion/Environment/VolumetricClouds/Resources/Materials/MPC_VolumetricClouds.MPC_VolumetricClouds" "Time" (Variables|Default|GetCloudsTime) :!class /Script/Engine.KismetMaterialLibrary))))

(fn RefreshSettings
  (bind _returnvalue (Math|Float|MakeLiteralFloat -5e+06))
  (bind _returnvalue_2 (Math|Float|MakeLiteralFloat 5e+06))
  (bind _returnvalue_3 (Math|Float|MultiplybyPi -2.0))
  (bind _cloudsbaseheight (Variables|Default|GetCloudsBaseHeight))
  (bind _directionalangle (Variables|Default|GetDirectionalAngle))
  (bind _cloudsscaleuniform (Variables|Default|GetCloudsScaleUniform))
  (bind _l_randomstream (LocalVariables|GetL_RandomStream))
  (bind _cloudcoverage (Variables|Default|GetCloudCoverage))
  (bind _returnvalue_4 (* _cloudcoverage _cloudcoverage))
  (bind _returnvalue_5 (+ _directionalangle 9e+01))
  (bind _returnvalue_6 (/ _returnvalue_5 3.6e+02))
  (bind _returnvalue_7 (* _returnvalue_6 _returnvalue_3))
  (Rendering|SetVisibility (Variables|Default|GetVolumetricCloud) (Variables|Default|GetEnabled) false)
  (if (Variables|Default|GetEnabled)
    (Utilities|FlowControl|Sequence
      (:then_0
        (Rendering|SetVisibility (Variables|Default|GetVolumetricCloud) (!= (or (== (Variables|Default|GetDensity) 0.0) (== (Variables|Default|GetCloudCoverage) 0.0)) true) false)
        (Class|VolumetricCloudComponent|SetTracingMaxDistance (Variables|Default|GetVolumetricCloud) (+ (* (Variables|Default|GetCloudsBaseHeight) 26.0) 115.0)))
      (:then_1
        (LocalVariables|SetL_CoverageCurveValue (Math|Curves|GetFloatValue (Variables|Default|GetCloudCoverageCurve) (Variables|Default|GetCloudCoverage)))
        (LocalVariables|SetL_CoveragePowValue (* _returnvalue_4 _returnvalue_4))
        (LocalVariables|SetL_CloudScaleCurve (* (+ (* _cloudsscaleuniform _cloudsscaleuniform) _cloudsscaleuniform) 0.5)))
      (:then_2
        (Class|VolumetricCloudComponent|SetLayerBottomAltitude (Variables|Default|GetVolumetricCloud) _cloudsbaseheight)
        (Class|VolumetricCloudComponent|SetLayerHeight (Variables|Default|GetVolumetricCloud) (* (Math|Float|Lerp 0.5 2.5 (LocalVariables|GetL_CloudScaleCurve)) (* (Variables|Default|GetCloudsScaleZ) 5.0)))
        (Rendering|Material|SetScalarParameterValue "/Game/Twinmotion/Environment/VolumetricClouds/Resources/Materials/MPC_VolumetricClouds.MPC_VolumetricClouds" "BottomHeight" _cloudsbaseheight :!class /Script/Engine.KismetMaterialLibrary)
        (Rendering|Material|SetScalarParameterValue "/Game/Twinmotion/Environment/VolumetricClouds/Resources/Materials/MPC_VolumetricClouds.MPC_VolumetricClouds" "Height" (* (Math|Float|Lerp 0.5 2.5 (LocalVariables|GetL_CloudScaleCurve)) (* (Variables|Default|GetCloudsScaleZ) 5.0)) :!class /Script/Engine.KismetMaterialLibrary)
        (Rendering|Material|SetScalarParameterValue "/Game/Twinmotion/Environment/VolumetricClouds/Resources/Materials/MPC_VolumetricClouds.MPC_VolumetricClouds" "CloudScaleZ" (Variables|Default|GetCloudsScaleZ) :!class /Script/Engine.KismetMaterialLibrary))
      (:then_3
        (Rendering|Material|SetScalarParameterValue "/Game/Twinmotion/Environment/VolumetricClouds/Resources/Materials/MPC_VolumetricClouds.MPC_VolumetricClouds" "CloudScale" (* (Math|Float|Lerp 0.25 1.25 (LocalVariables|GetL_CloudScaleCurve)) 1e+07) :!class /Script/Engine.KismetMaterialLibrary)
        (Rendering|Material|SetScalarParameterValue "/Game/Twinmotion/Environment/VolumetricClouds/Resources/Materials/MPC_VolumetricClouds.MPC_VolumetricClouds" "CloudDetailScale" (Math|Float|Lerp 2e+06 3e+06 (LocalVariables|GetL_CloudScaleCurve)) :!class /Script/Engine.KismetMaterialLibrary)
        (Rendering|Material|SetScalarParameterValue "/Game/Twinmotion/Environment/VolumetricClouds/Resources/Materials/MPC_VolumetricClouds.MPC_VolumetricClouds" "CloudsScaleNormalized" (LocalVariables|GetL_CloudScaleCurve) :!class /Script/Engine.KismetMaterialLibrary))
      (:then_4
        (Rendering|Material|SetScalarParameterValue "/Game/Twinmotion/Environment/VolumetricClouds/Resources/Materials/MPC_VolumetricClouds.MPC_VolumetricClouds" "WispsStrength" (Variables|Default|GetWispyness) :!class /Script/Engine.KismetMaterialLibrary)
        (Rendering|Material|SetScalarParameterValue "/Game/Twinmotion/Environment/VolumetricClouds/Resources/Materials/MPC_VolumetricClouds.MPC_VolumetricClouds" "CloudCoverage" (LocalVariables|GetL_CoverageCurveValue) :!class /Script/Engine.KismetMaterialLibrary)
        (Rendering|Material|SetScalarParameterValue "/Game/Twinmotion/Environment/VolumetricClouds/Resources/Materials/MPC_VolumetricClouds.MPC_VolumetricClouds" "RoundBottom" (* (- 1.0 (Variables|Default|GetFlatBottom)) 0.5) :!class /Script/Engine.KismetMaterialLibrary)
        (Rendering|Material|SetScalarParameterValue "/Game/Twinmotion/Environment/VolumetricClouds/Resources/Materials/MPC_VolumetricClouds.MPC_VolumetricClouds" "Density" (Variables|Default|GetDensity) :!class /Script/Engine.KismetMaterialLibrary)
        (Rendering|Material|SetScalarParameterValue "/Game/Twinmotion/Environment/VolumetricClouds/Resources/Materials/MPC_VolumetricClouds.MPC_VolumetricClouds" "NearDissipationAmount" (Variables|Default|GetNearDissipation) :!class /Script/Engine.KismetMaterialLibrary)
        (Rendering|Material|SetScalarParameterValue "/Game/Twinmotion/Environment/VolumetricClouds/Resources/Materials/MPC_VolumetricClouds.MPC_VolumetricClouds" "NimbusAmount" (Variables|Default|GetPuffyness) :!class /Script/Engine.KismetMaterialLibrary)
        (Rendering|Material|SetScalarParameterValue "/Game/Twinmotion/Environment/VolumetricClouds/Resources/Materials/MPC_VolumetricClouds.MPC_VolumetricClouds" "NearDissipationRadius" (Math|Float|Max(Float) (* (Variables|Default|GetNearDissipationRadius) 1e+05) 0.01) :!class /Script/Engine.KismetMaterialLibrary)
        (Rendering|Material|SetVectorParameterValue "/Game/Twinmotion/Environment/VolumetricClouds/Resources/Materials/MPC_VolumetricClouds.MPC_VolumetricClouds" "DirectionalHole" (Utilities|Struct|MakeLinearColor (Variables|Default|GetDirectionalDissipation) (Math|Trig|Sin(Radians) _returnvalue_7) (Math|Trig|Cos(Radians) _returnvalue_7) 0.0) :!class /Script/Engine.KismetMaterialLibrary)
        (Rendering|Material|SetVectorParameterValue "/Game/Twinmotion/Environment/VolumetricClouds/Resources/Materials/MPC_VolumetricClouds.MPC_VolumetricClouds" "Albedo" (Variables|Default|GetAlbedo) :!class /Script/Engine.KismetMaterialLibrary))
      (:then_5
        (Variables|Default|SetStaticOffset (* (Variables|Default|GetManualOffset) 1e+05))
        (Math|Random|SetRandomStreamSeed _l_randomstream (Variables|Default|GetRandomSeed))
        (Rendering|Material|SetVectorParameterValue "/Game/Twinmotion/Environment/VolumetricClouds/Resources/Materials/MPC_VolumetricClouds.MPC_VolumetricClouds" "RandomOffset" (Utilities|Struct|MakeLinearColor (Math|Random|RandomFloatinRangefromStream _l_randomstream _returnvalue _returnvalue_2) (Math|Random|RandomFloatinRangefromStream _l_randomstream _returnvalue _returnvalue_2) (Math|Random|RandomFloatinRangefromStream _l_randomstream _returnvalue _returnvalue_2) (Math|Random|RandomFloatinRangefromStream _l_randomstream _returnvalue _returnvalue_2)) :!class /Script/Engine.KismetMaterialLibrary))
      (:then_6
        (Rendering|Material|SetScalarParameterValue "/Game/Twinmotion/Environment/VolumetricClouds/Resources/Materials/MPC_VolumetricClouds.MPC_VolumetricClouds" "SkydomeCloudCoverage" (Variables|Default|GetEnableCirrus) :!class /Script/Engine.KismetMaterialLibrary)))))

(fn Hash1in4out
  (params (Seed :type Integer))
  (bind _returnvalue (Math|Float|MakeLiteralFloat 33.33))
  (LocalVariables|SetL_p (Math|Float|MultiplybyPi (Math|Conversions|ToFloat(Integer) Seed)))
  (Utilities|FlowControl|Sequence
    (:then_0
      (LocalVariables|SetL_p4 (* (Math|Float|Fraction (LocalVariables|GetL_p)) (Utilities|Struct|MakeLinearColor 0.1031 0.103 0.0973 0.1099))))
    (:then_1
      (LocalVariables|SetL_p4 (+ (LocalVariables|GetL_p4) (Class|KismetMathLibrary|Vector4DotProduct (Math|Vector4|MakeVector4 (.r (LocalVariables|GetL_p4)) (.g (LocalVariables|GetL_p4)) (.b (LocalVariables|GetL_p4)) (.a (LocalVariables|GetL_p4))) (+ (Math|Vector4|MakeVector4 (.a (LocalVariables|GetL_p4)) (.r (LocalVariables|GetL_p4)) (.g (LocalVariables|GetL_p4)) (.b (LocalVariables|GetL_p4))) (Math|Vector4|MakeVector4 _returnvalue _returnvalue _returnvalue _returnvalue))))))
    (:then_2
      (return (* (- (Utilities|Struct|MakeLinearColor (Math|Float|Fraction (.r (* (+ (Utilities|Struct|MakeLinearColor (.r (LocalVariables|GetL_p4)) (.r (LocalVariables|GetL_p4)) (.g (LocalVariables|GetL_p4)) (.b (LocalVariables|GetL_p4))) (Utilities|Struct|MakeLinearColor (.g (LocalVariables|GetL_p4)) (.b (LocalVariables|GetL_p4)) (.b (LocalVariables|GetL_p4)) (.a (LocalVariables|GetL_p4)))) (Utilities|Struct|MakeLinearColor (.b (LocalVariables|GetL_p4)) (.g (LocalVariables|GetL_p4)) (.a (LocalVariables|GetL_p4)) (.r (LocalVariables|GetL_p4)))))) (Math|Float|Fraction (.g (* (+ (Utilities|Struct|MakeLinearColor (.r (LocalVariables|GetL_p4)) (.r (LocalVariables|GetL_p4)) (.g (LocalVariables|GetL_p4)) (.b (LocalVariables|GetL_p4))) (Utilities|Struct|MakeLinearColor (.g (LocalVariables|GetL_p4)) (.b (LocalVariables|GetL_p4)) (.b (LocalVariables|GetL_p4)) (.a (LocalVariables|GetL_p4)))) (Utilities|Struct|MakeLinearColor (.b (LocalVariables|GetL_p4)) (.g (LocalVariables|GetL_p4)) (.a (LocalVariables|GetL_p4)) (.r (LocalVariables|GetL_p4)))))) (Math|Float|Fraction (.b (* (+ (Utilities|Struct|MakeLinearColor (.r (LocalVariables|GetL_p4)) (.r (LocalVariables|GetL_p4)) (.g (LocalVariables|GetL_p4)) (.b (LocalVariables|GetL_p4))) (Utilities|Struct|MakeLinearColor (.g (LocalVariables|GetL_p4)) (.b (LocalVariables|GetL_p4)) (.b (LocalVariables|GetL_p4)) (.a (LocalVariables|GetL_p4)))) (Utilities|Struct|MakeLinearColor (.b (LocalVariables|GetL_p4)) (.g (LocalVariables|GetL_p4)) (.a (LocalVariables|GetL_p4)) (.r (LocalVariables|GetL_p4)))))) (Math|Float|Fraction (.a (* (+ (Utilities|Struct|MakeLinearColor (.r (LocalVariables|GetL_p4)) (.r (LocalVariables|GetL_p4)) (.g (LocalVariables|GetL_p4)) (.b (LocalVariables|GetL_p4))) (Utilities|Struct|MakeLinearColor (.g (LocalVariables|GetL_p4)) (.b (LocalVariables|GetL_p4)) (.b (LocalVariables|GetL_p4)) (.a (LocalVariables|GetL_p4)))) (Utilities|Struct|MakeLinearColor (.b (LocalVariables|GetL_p4)) (.g (LocalVariables|GetL_p4)) (.a (LocalVariables|GetL_p4)) (.r (LocalVariables|GetL_p4))))))) 0.5) 1e+07)))))