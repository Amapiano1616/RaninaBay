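; Blueprint that advances the global wind position stored in a Material Parameter Collection.
; Each tick it reads the wind direction and vegetation wind speed from the collection and adds their product, scaled by delta time, to the stored position.
; When the Twinmotion paused parameter is set, speed becomes zero, so the accumulated position holds still.
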(event EventTick
  (params (DeltaSeconds :type Float%20%28single-precision%29))
  (bind _returnvalue (Rendering|Material|GetVectorParameterValue (Variables|Default|GetMPC) (Utilities|Name|MakeLiteralName "CPV3_GlobalWindPosition") :!class /Script/Engine.KismetMaterialLibrary))
  (bind _returnvalue_2 (Rendering|Material|GetVectorParameterValue (Variables|Default|GetMPC) (Utilities|Name|MakeLiteralName "CPV3_WindDirection") :!class /Script/Engine.KismetMaterialLibrary))
  (bind _returnvalue_3 (Rendering|Material|GetScalarParameterValue (Variables|Default|GetMPC) (Utilities|Name|MakeLiteralName "CPS_TwinmotionPaused") :!class /Script/Engine.KismetMaterialLibrary))
  (bind _returnvalue_4 (Rendering|Material|GetScalarParameterValue (Variables|Default|GetMPC) (Utilities|Name|MakeLiteralName "CPS_VegetationWindSpeed") :!class /Script/Engine.KismetMaterialLibrary))
  (Rendering|Material|SetVectorParameterValue (Variables|Default|GetMPC) (Utilities|Name|MakeLiteralName "CPV3_GlobalWindPosition") (Math|Conversions|ToLinearColor(Vector) (+ (Math|Conversions|ToVector(LinearColor) _returnvalue) (* (Math|Conversions|ToVector(LinearColor) _returnvalue_2) (Math|Float|SelectFloat 0.0 _returnvalue_4 (> _returnvalue_3 0.5)) DeltaSeconds))) :!class /Script/Engine.KismetMaterialLibrary))